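; BP_BaseSida1 is a base Blueprint for the IDA1 product that turns keyboard input into directional key events.
; W, S, A, D and the Up/Down arrows call handler functions defined outside this graph, passing Pressed and Released flags.
; D maps to OnLeftKey and A to OnRightKey, the reverse of the usual layout.
; Tick and the construction script are empty, so the graph only forwards input.
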(event EventBeginPlay)

(event Collision|EventActorBeginOverlap
  (params (OtherActor :type Actor%20Object%20Reference)))

(event EventTick
  (params (DeltaSeconds :type Float%20%28single-precision%29)))

(event Input|KeyboardEvents|D
  (params (Key :type Key%20Structure :default "None"))
  (:Released
    (Class|CBoatBase|OnLeftKey false true)))

(event Input|KeyboardEvents|W
  (params (Key :type Key%20Structure :default "None"))
  (:Pressed
    (Class|CBoatBase|OnForwardKey true false))
  (:Released
    (Class|CBoatBase|OnForwardKey false true)))

(event Input|KeyboardEvents|S
  (params (Key :type Key%20Structure :default "None"))
  (:Pressed
    (Class|CBoatBase|OnBackwardkKey true false))
  (:Released
    (Class|CBoatBase|OnBackwardkKey false true)))

(event Input|KeyboardEvents|Down
  (params (Key :type Key%20Structure :default "None"))
  (:Released
    (Class|CBoatBase|OnDownKeyPressed false true)))

(event Input|KeyboardEvents|D
  (params (Key :type Key%20Structure :default "None"))
  (:Pressed
    (Class|CBoatBase|OnLeftKey true false)))

(event Input|KeyboardEvents|A
  (params (Key :type Key%20Structure :default "None"))
  (:Pressed
    (Class|CBoatBase|OnRightKey true false)))

(event Input|KeyboardEvents|A
  (params (Key :type Key%20Structure :default "None"))
  (:Released
    (Class|CBoatBase|OnRightKey false true)))

(event Input|KeyboardEvents|Up
  (params (Key :type Key%20Structure :default "None"))
  (:Pressed
    (Class|CBoatBase|OnUpKeyPressed true false)))

(event Input|KeyboardEvents|Up
  (params (Key :type Key%20Structure :default "None"))
  (:Released
    (Class|CBoatBase|OnUpKeyPressed false true)))

(event Input|KeyboardEvents|Down
  (params (Key :type Key%20Structure :default "None"))
  (:Pressed
    (Class|CBoatBase|OnDownKeyPressed true false)))

(fn ConstructionScript)