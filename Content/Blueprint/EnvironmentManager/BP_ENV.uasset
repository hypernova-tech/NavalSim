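; Environment manager Blueprint that pushes weather, time-of-day and wind settings to the UDS sky, UDW weather and Ocean references every Tick.
; Getter values are range-mapped into UDW weather levels and UDS time and fog intensity, while sky scattering color passes straight through.
; Ocean receives FFT wind and tracks the player pawn.
; Both ocean-dirty branches enable the dynamic environment, and the fog inscattering color update is unconnected.
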(event EventBeginPlay)

(event Collision|EventActorBeginOverlap
  (params (OtherActor :type Actor%20Object%20Reference)))

(event EventTick
  (params (DeltaSeconds :type Float%20%28single-precision%29))
  (bind _udw (Variables|Default|GetUDW))
  (bind _ocean (Variables|Default|GetOcean))
  (bind _ocean_2 (Variables|Default|GetOcean))
  (bind _udw_2 (Variables|Default|GetUDW))
  (bind _returnvalue (Class|EnvManager|GetIsOceanDynamicsDirty))
  (if _returnvalue
    (Variables|/Game/Waterline/3_Ocean_Sim_Content/BP_Waterline_Ocean_Gen_3.BP_Waterline_Ocean_Gen_3_C|SetDynamic%20Ocean%20Environment _ocean_2 true)
    (else
      (Variables|/Game/Waterline/3_Ocean_Sim_Content/BP_Waterline_Ocean_Gen_3.BP_Waterline_Ocean_Gen_3_C|SetDynamic%20Ocean%20Environment _ocean_2 true)))
  (bind _returnvalue_2 (Class|EnvManager|GetRainLevelPercent))
  (Variables|/Game/UltraDynamicSky/Blueprints/Ultra_Dynamic_Weather.Ultra_Dynamic_Weather_C|SetRain _udw_2 (Math|Float|MapRangeClamped _returnvalue_2 0.0 1e+02 0.0 1e+01))
  (bind _returnvalue_3 (Class|EnvManager|GetCloudLevelPercent))
  (Variables|/Game/UltraDynamicSky/Blueprints/Ultra_Dynamic_Weather.Ultra_Dynamic_Weather_C|SetCloud%20Coverage _udw_2 (Math|Float|MapRangeClamped _returnvalue_3 0.0 1e+02 0.0 1e+01))
  (bind _returnvalue_4 (Class|EnvManager|GetSnowLevelPercent))
  (Variables|/Game/UltraDynamicSky/Blueprints/Ultra_Dynamic_Weather.Ultra_Dynamic_Weather_C|SetSnow _udw_2 (Math|Float|MapRangeClamped _returnvalue_4 0.0 1e+02 0.0 1e+01))
  (bind _returnvalue_5 (Class|EnvManager|GetDustLevelPercent))
  (Variables|/Game/UltraDynamicSky/Blueprints/Ultra_Dynamic_Weather.Ultra_Dynamic_Weather_C|SetDust _udw_2 (Math|Float|MapRangeClamped _returnvalue_5 0.0 1e+02 0.0 1e+01))
  (bind _returnvalue_6 (Class|EnvManager|GetThunderLevelPercent))
  (Variables|/Game/UltraDynamicSky/Blueprints/Ultra_Dynamic_Weather.Ultra_Dynamic_Weather_C|SetThunder/Lightning _udw_2 (Math|Float|MapRangeClamped _returnvalue_6 0.0 1e+02 0.0 1e+01))
  (bind _returnvalue_7 (Class|EnvManager|GetFogLevelPercent))
  (Variables|/Game/UltraDynamicSky/Blueprints/Ultra_Dynamic_Weather.Ultra_Dynamic_Weather_C|SetFog _udw_2 (Math|Float|MapRangeClamped _returnvalue_7 0.0 1e+02 0.0 1e+01))
  (bind _returnvalue_8 (Class|EnvManager|GetTimeOfDayHr))
  (bind _returnvalue_9 (Class|EnvManager|GetFogColorIntensity))
  (Variables|/Game/UltraDynamicSky/Blueprints/Ultra_Dynamic_Sky.Ultra_Dynamic_Sky_C|SetFog%20Color%20Intensity%20Scale (Variables|Default|GetUDS) (Math|Float|MapRangeClamped _returnvalue_7 0.0 1e+02 (.X (Math|Vector|BreakVector (Math|Conversions|ToVector(Vector2D) _returnvalue_9))) (.Y (Math|Vector|BreakVector (Math|Conversions|ToVector(Vector2D) _returnvalue_9)))))
  (Variables|/Game/UltraDynamicSky/Blueprints/Ultra_Dynamic_Sky.Ultra_Dynamic_Sky_C|SetTime%20of%20Day (Variables|Default|GetUDS) (Math|Float|MapRangeClamped _returnvalue_8 0.0 24.0 0.0 2.4e+03))
  (bind _returnvalue_10 (Class|EnvManager|GetWindDirectionDeg))
  (Variables|/Game/UltraDynamicSky/Blueprints/Ultra_Dynamic_Weather.Ultra_Dynamic_Weather_C|SetWind%20Direction _udw _returnvalue_10)
  (bind _returnvalue_11 (Class|EnvManager|GetWindSpeedMetersPerSec))
  (Variables|/Game/UltraDynamicSky/Blueprints/Ultra_Dynamic_Weather.Ultra_Dynamic_Weather_C|SetWind%20Intensity _udw (Math|Float|MapRangeClamped _returnvalue_11 0.0 1e+02 0.0 3e+01))
  (Variables|/Game/Waterline/3_Ocean_Sim_Content/BP_Waterline_Ocean_Gen_3.BP_Waterline_Ocean_Gen_3_C|SetWind%20Speed%20FFT _ocean _returnvalue_11)
  (bind _returnvalue_12 (Class|EnvManager|GetWindDirectionVector))
  (Variables|/Game/Waterline/3_Ocean_Sim_Content/BP_Waterline_Ocean_Gen_3.BP_Waterline_Ocean_Gen_3_C|SetWind%20Direction%20FFT _ocean _returnvalue_12)
  (Variables|/Game/Waterline/3_Ocean_Sim_Content/BP_Waterline_Ocean_Gen_3.BP_Waterline_Ocean_Gen_3_C|SetTrack%20Actor _ocean (Pawn|GetControlledPawn (Game|GetPlayerController 0)))
  (bind _returnvalue_13 (Class|EnvManager|GetRayleighScatteringColorDay))
  (Variables|/Game/UltraDynamicSky/Blueprints/Ultra_Dynamic_Sky.Ultra_Dynamic_Sky_C|SetRayleigh%20Scattering%20Color%20%28Day%29 (Variables|Default|GetUDS) _returnvalue_13))

(fn ConstructionScript)