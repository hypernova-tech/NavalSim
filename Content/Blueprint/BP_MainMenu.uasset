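; Main menu actor that puts a BP_UI control panel on screen for tuning an ocean and boat scene.
; On BeginPlay it creates the widget and registers its images as three lidar and five camera display slots.
; Tick polls sliders and checkboxes to drive ocean wind, waves and foam, Ulaq's speed, sun pitch, and cloud and fog visibility.
; A Space bar debug key toggles the panel and mouse cursor.
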(event EventBeginPlay
  (bind _returnvalue (Game|GetPlayerController 0))
  (Input|EnableInput _returnvalue)
  (bind _returnvalue_2 (UserInterface|CreateWidget "/Game/Blueprint/BP_UI.BP_UI_C" _returnvalue))
  (Variables|Default|SetUIWidget _returnvalue_2)
  (UserInterface|Viewport|AddtoViewport (Variables|Default|GetUIWidget) 0)
  (Class|UIControllerBase|SetLidarSlotImage 0 (Variables|/Game/Blueprint/BP_UI.BP_UI_C|GetImageLidar1 (Variables|Default|GetUIWidget)))
  (Class|UIControllerBase|SetLidarSlotImage 1 (Variables|/Game/Blueprint/BP_UI.BP_UI_C|GetImageLidar2 (Variables|Default|GetUIWidget)))
  (Class|UIControllerBase|SetLidarSlotImage 2 (Variables|/Game/Blueprint/BP_UI.BP_UI_C|GetImageLidar3 (Variables|Default|GetUIWidget)))
  (Class|UIControllerBase|SetCameraSlotImage 0 (Variables|/Game/Blueprint/BP_UI.BP_UI_C|GetCameraSlot1 (Variables|Default|GetUIWidget)))
  (Class|UIControllerBase|SetCameraSlotImage 1 (Variables|/Game/Blueprint/BP_UI.BP_UI_C|GetCameraSlot2 (Variables|Default|GetUIWidget)))
  (Class|UIControllerBase|SetCameraSlotImage 2 (Variables|/Game/Blueprint/BP_UI.BP_UI_C|GetCameraSlot3 (Variables|Default|GetUIWidget)))
  (Class|UIControllerBase|SetCameraSlotImage 3 (Variables|/Game/Blueprint/BP_UI.BP_UI_C|GetCameraSlot4 (Variables|Default|GetUIWidget)))
  (Class|UIControllerBase|SetCameraSlotImage 4 (Variables|/Game/Blueprint/BP_UI.BP_UI_C|GetCameraSlot5 (Variables|Default|GetUIWidget))))

(event Collision|EventActorBeginOverlap
  (params (OtherActor :type Actor%20Object%20Reference)))

(event EventTick
  (params (DeltaSeconds :type Float%20%28single-precision%29))
  (bind _ocean (Variables|Default|GetOcean))
  (bind _uiwidget (Variables|Default|GetUIWidget))
  (Variables|/Game/Waterline/3_Ocean_Sim_Content/BP_Waterline_Ocean_Gen_3.BP_Waterline_Ocean_Gen_3_C|SetWind%20Speed%20FFT _ocean (Class|Slider|GetValue (Variables|/Game/Blueprint/BP_UI.BP_UI_C|GetSliderWind _uiwidget)))
  (Variables|/Script/BoatSim.CBoatBase|SetMovementSpeedUnitPerSec (Variables|Default|GetUlaq) (Class|Slider|GetValue (Variables|/Game/Blueprint/BP_UI.BP_UI_C|GetSliderBoatSpeed _uiwidget)))
  (Variables|/Game/Waterline/3_Ocean_Sim_Content/BP_Waterline_Ocean_Gen_3.BP_Waterline_Ocean_Gen_3_C|SetSimulation%20Height _ocean (Class|Slider|GetValue (Variables|/Game/Blueprint/BP_UI.BP_UI_C|GetSliderWaveHeight _uiwidget)))
  (Variables|/Game/Waterline/3_Ocean_Sim_Content/BP_Waterline_Ocean_Gen_3.BP_Waterline_Ocean_Gen_3_C|SetDynamic%20Foam _ocean (Class|CheckBox|IsChecked (Variables|/Game/Blueprint/BP_UI.BP_UI_C|GetUseFoamCb _uiwidget)))
  (Variables|/Game/Waterline/3_Ocean_Sim_Content/BP_Waterline_Ocean_Gen_3.BP_Waterline_Ocean_Gen_3_C|SetFoam%20WhiteCaps%20Power _ocean (Class|Slider|GetValue (Variables|/Game/Blueprint/BP_UI.BP_UI_C|GetSliderFoam _uiwidget)))
  (Transformation|SetWorldRotation (Variables|/Script/Engine.Actor|GetRootComponent (Variables|Default|GetSun)) (Math|Rotator|MakeRotator 0.0 (Variables|/Script/UMG.Slider|GetValue (Variables|/Game/Blueprint/BP_UI.BP_UI_C|GetSunLocationSlider _uiwidget)) 0.0) false false)
  (Rendering|SetActorHiddenInGame (Variables|Default|GetCloud) (not (Class|CheckBox|IsChecked (Variables|/Game/Blueprint/BP_UI.BP_UI_C|GetUseCloudCB _uiwidget))))
  (Rendering|SetActorHiddenInGame (Variables|Default|GetFog) (not (Class|CheckBox|IsChecked (Variables|/Game/Blueprint/BP_UI.BP_UI_C|GetUseFogCB _uiwidget)))))

(event Input|KeyboardEvents|DebugKeySpaceBar
  (params (Key :type Key%20Structure :default "None") (ActionValue :type Input%20Action%20Value%20Structure))
  (bind _returnvalue (Game|GetPlayerController 0))
  (bind _uiwidget (Variables|Default|GetUIWidget))
  (:Pressed
    (Utilities|FlowControl|FlipFlop
      (:A
        (Variables|/Script/UMG.Widget|SetVisibility _uiwidget "Visible")
        (Input|SetInputModeGameandUI _returnvalue 0 "DoNotLock" false false)
        (Variables|/Script/Engine.PlayerController|SetbShowMouseCursor _returnvalue true))
      (:B
        (Variables|/Script/UMG.Widget|SetVisibility _uiwidget "Hidden")
        (Input|SetInputModeGameandUI 0 0 "DoNotLock" false false)
        (Variables|/Script/Engine.PlayerController|SetbShowMouseCursor _returnvalue false)))))

(fn ConstructionScript)