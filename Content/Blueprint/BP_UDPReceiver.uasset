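; UDP receiver actor that listens on a hardcoded port and hands incoming packets to the level's SOAImplementor actor.
; BeginPlay finds and caches that actor, then starts the socket only if the cast succeeds.
; Tick polls the packet queue in a bounded loop of about a hundred passes, passing each available packet to OnReceivedNewMessage to cap per-frame work.
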(event EventBeginPlay
  (bind _returnvalue (Actor|GetActorOfClass "/Script/BoatSim.SOAImplementor"))
  (bind _assoaimplementor (Utilities|Casting|CastToSOAImplementor _returnvalue))
  (Variables|Default|SetAs%20SOAImplementor _assoaimplementor)
  (Class|UDPReceiver|StartUDPReceiver "fdf" 22333)
  (Development|PrintString (Utilities|String|ToString(Integer) 0) true true "(R=0.000000,G=0.660000,B=1.000000,A=1.000000)" 0.5))

(event Collision|EventActorBeginOverlap
  (params (OtherActor :type Actor%20Object%20Reference)))

(event EventTick
  (params (DeltaSeconds :type Float%20%28single-precision%29))
  (for _index (range 0 100)
    (bind _returnvalue (Class|UDPReceiver|GetReceivedPacketCount))
    (Math|Integer|CompareInt _returnvalue
      (:>
        (bind _returnvalue_2 (Class|UDPReceiver|GetNextPacket))
        (Class|SOAImplementor|OnReceivedNewMessage (Variables|Default|GetAs%20SOAImplementor) _returnvalue_2)))))

(fn ConstructionScript)