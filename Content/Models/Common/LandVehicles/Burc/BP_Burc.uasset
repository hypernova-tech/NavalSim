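; BP_Burc is a land vehicle Blueprint with a gun and separate turret, gun and electro-optical (EO) gimbals.
; Its construction script stores the gun tip and weapon (Silah) components in P-prefixed variables, then casts the three gimbal child actors to GimbalBase and caches them likewise.
; The casts run in sequence, so a failed one leaves the remaining gimbal references unset.
; The event graph holds no active logic.
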(event Collision|EventActorBeginOverlap
  (params (OtherActor :type Actor%20Object%20Reference)))

(event EventTick
  (params (DeltaSeconds :type Float%20%28single-precision%29)))

(fn ConstructionScript
  (Variables|Default|SetpGunTip (Variables|Default|GetTipOfGun))
  (Variables|Default|SetpGun (Variables|Default|GetSilah))
  (bind _asgimbal_base (Utilities|Casting|CastToGimbalBase (Variables|/Script/Engine.ChildActorComponent|GetChildActor (Variables|Default|GetTaretGimbal))))
  (Variables|Default|SetpTaretGimbal _asgimbal_base)
  (bind _asgimbal_base_2 (Utilities|Casting|CastToGimbalBase (Variables|/Script/Engine.ChildActorComponent|GetChildActor (Variables|Default|GetGunGimbal))))
  (Variables|Default|SetpGunGimbal _asgimbal_base_2)
  (bind _asgimbal_base_3 (Utilities|Casting|CastToGimbalBase (Variables|/Script/Engine.ChildActorComponent|GetChildActor (Variables|Default|GetEOGimbal))))
  (Variables|Default|SetpEOGimbal _asgimbal_base_3))