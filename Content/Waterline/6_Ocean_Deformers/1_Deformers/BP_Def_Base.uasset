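; Base ocean deformer actor for the Waterline system, carrying a virtual texture volume sized by Scale and Height.
; The construction script places the actor at its configured XY location, makes the volume movable and offsets it by half its scale.
; With InfiniteScaleDynamicLocation enabled, it snaps to the ocean generator's WaterPlane and reapplies that offset on BeginPlay, Box1 overlap end or CenterActor.
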(event OnComponentEndOverlap(Box1)
  (params (OverlappedComponent :type Primitive%20Component%20Object%20Reference) (OtherActor :type Actor%20Object%20Reference) (OtherComp :type Primitive%20Component%20Object%20Reference) (OtherBodyIndex :type Integer))
  (bind _virtualtexturecomponent (Variables|Default|GetVirtualTextureComponent))
  (if (Variables|Default|GetInfinite%20Scale%20%28Dynamic%20Location%29)
    (Utilities|FlowControl|DoOnce false :!label _label
      (:Completed
        (bind _returnvalue (Actor|GetActorOfClass "/Game/Waterline/3_Ocean_Sim_Content/BP_Waterline_Ocean_Gen_3.BP_Waterline_Ocean_Gen_3_C"))
        (Transformation|SetActorLocation (Transformation|GetWorldLocation (Variables|/Game/Waterline/3_Ocean_Sim_Content/BP_Waterline_Ocean_Gen_3.BP_Waterline_Ocean_Gen_3_C|GetWaterPlane _returnvalue)) false false)
        (Transformation|AddLocalOffset _virtualtexturecomponent (/ (Transformation|GetWorldScale _virtualtexturecomponent) -2.0) false false)
        (goto _label Reset)))))

(event Custom|Center%20Actor
  (bind _virtualtexturecomponent (Variables|Default|GetVirtualTextureComponent))
  (if (Variables|Default|GetInfinite%20Scale%20%28Dynamic%20Location%29)
    (Utilities|FlowControl|DoOnce false :!label _label
      (:Completed
        (bind _returnvalue (Actor|GetActorOfClass "/Game/Waterline/3_Ocean_Sim_Content/BP_Waterline_Ocean_Gen_3.BP_Waterline_Ocean_Gen_3_C"))
        (Transformation|SetActorLocation (Transformation|GetWorldLocation (Variables|/Game/Waterline/3_Ocean_Sim_Content/BP_Waterline_Ocean_Gen_3.BP_Waterline_Ocean_Gen_3_C|GetWaterPlane _returnvalue)) false false)
        (Transformation|AddLocalOffset _virtualtexturecomponent (/ (Transformation|GetWorldScale _virtualtexturecomponent) -2.0) false false)
        (goto _label Reset)))))

(event EventBeginPlay
  (bind _virtualtexturecomponent (Variables|Default|GetVirtualTextureComponent))
  (Utilities|FlowControl|Delay 0.0)
  (if (Variables|Default|GetInfinite%20Scale%20%28Dynamic%20Location%29)
    (Utilities|FlowControl|DoOnce false :!label _label
      (:Completed
        (bind _returnvalue (Actor|GetActorOfClass "/Game/Waterline/3_Ocean_Sim_Content/BP_Waterline_Ocean_Gen_3.BP_Waterline_Ocean_Gen_3_C"))
        (Transformation|SetActorLocation (Transformation|GetWorldLocation (Variables|/Game/Waterline/3_Ocean_Sim_Content/BP_Waterline_Ocean_Gen_3.BP_Waterline_Ocean_Gen_3_C|GetWaterPlane _returnvalue)) false false)
        (Transformation|AddLocalOffset _virtualtexturecomponent (/ (Transformation|GetWorldScale _virtualtexturecomponent) -2.0) false false)
        (goto _label Reset)))))

(fn ConstructionScript
  (bind _virtualtexturecomponent (Variables|Default|GetVirtualTextureComponent))
  (bind _scale (Variables|Default|GetScale))
  (Transformation|SetWorldScale3D _virtualtexturecomponent (Math|Vector|MakeVector _scale _scale (Variables|Default|GetHeight)))
  (Transformation|SetActorLocation (Math|Vector|MakeVector (Variables|Default|GetLocation%20X) (Variables|Default|GetNew%20Location%20Y) 0.0) false false)
  (Transformation|AddLocalOffset _virtualtexturecomponent (/ (Transformation|GetWorldScale _virtualtexturecomponent) -2.0) false false)
  (Transformation|SetMobility _virtualtexturecomponent "Movable"))