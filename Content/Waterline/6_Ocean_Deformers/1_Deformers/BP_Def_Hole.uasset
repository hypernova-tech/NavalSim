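; Waterline ocean deformer for a hole in the water, where the underwater post-process is switched off while the player is inside.
; The construction script gives the inner shell the DeformerShape mesh and an inner glass-wall material.
; Shell overlaps by the player pawn toggle the UnderwaterPostProcessVolume on BP_Waterline_Ocean_Gen_3.
; BeginPlay shares the disable step when already overlapped, though only begin-overlap looks up the ocean actor.
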(event OnComponentBeginOverlap(Shell_Inner)
  (params (OverlappedComponent :type Primitive%20Component%20Object%20Reference) (OtherActor :type Actor%20Object%20Reference) (OtherComp :type Primitive%20Component%20Object%20Reference) (OtherBodyIndex :type Integer) (bFromSweep :type Boolean) (SweepResult :type Hit%20Result%20Structure%20%28by%20ref%29))
  (if (== OtherActor (Game|Player|GetPlayerPawn 0))
    (bind _returnvalue (Actor|GetActorOfClass "/Game/Waterline/3_Ocean_Sim_Content/BP_Waterline_Ocean_Gen_3.BP_Waterline_Ocean_Gen_3_C"))
    (Variables|/Script/Engine.PostProcessComponent|SetbEnabled (Variables|/Game/Waterline/3_Ocean_Sim_Content/BP_Waterline_Ocean_Gen_3.BP_Waterline_Ocean_Gen_3_C|GetUnderwater%20Post-Process%20Volume _returnvalue) false)))

(event OnComponentEndOverlap(Shell_Inner)
  (params (OverlappedComponent :type Primitive%20Component%20Object%20Reference) (OtherActor :type Actor%20Object%20Reference) (OtherComp :type Primitive%20Component%20Object%20Reference) (OtherBodyIndex :type Integer))
  (if (== OtherActor (Game|Player|GetPlayerPawn 0))
    (bind _returnvalue (Actor|GetActorOfClass "/Game/Waterline/3_Ocean_Sim_Content/BP_Waterline_Ocean_Gen_3.BP_Waterline_Ocean_Gen_3_C"))
    (Variables|/Script/Engine.PostProcessComponent|SetbEnabled (Variables|/Game/Waterline/3_Ocean_Sim_Content/BP_Waterline_Ocean_Gen_3.BP_Waterline_Ocean_Gen_3_C|GetUnderwater%20Post-Process%20Volume _returnvalue) true)))

(event EventBeginPlay
  (bind _returnvalue (Game|Player|GetPlayerPawn 0))
  (if (Utilities|Array|ContainsItem (Collision|GetOverlappingActors (Utilities|GetClass _returnvalue) :!class /Script/Engine.Actor) _returnvalue)
    (Variables|/Script/Engine.PostProcessComponent|SetbEnabled (Variables|/Game/Waterline/3_Ocean_Sim_Content/BP_Waterline_Ocean_Gen_3.BP_Waterline_Ocean_Gen_3_C|GetUnderwater%20Post-Process%20Volume (stale OnComponentBeginOverlap(Shell_Inner) _returnvalue)) false)))

(fn ConstructionScript
  (Components|StaticMesh|SetStaticMesh (Variables|Default|GetShell_Inner) (Variables|Default|GetDeformer%20Shape))
  (Rendering|Material|SetMaterial (Variables|Default|GetShell_Inner) 0 "/Game/Waterline/6_Ocean_Deformers/2_Materials/M_Def_Glass_Wall_In.M_Def_Glass_Wall_In"))