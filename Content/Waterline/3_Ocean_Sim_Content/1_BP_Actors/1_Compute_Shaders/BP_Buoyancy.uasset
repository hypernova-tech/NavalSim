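; Buoyancy actor prototype for the Waterline ocean sim, currently inert: every event and the construction script are empty, and all logic is disconnected.
; The disconnected graphs rebuild a procedural collision grid from Niagara particle data and collect overlapping physics primitives, optionally filtered by a "Float" tag.
; Each primitive's position wraps into one ocean tile for a line trace against that grid, whose hit drives mass-scaled lift, normal-based drift and damping.
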(event OnComponentBeginOverlap(BuoyancyVolume)
  (params (OverlappedComponent :type Primitive%20Component%20Object%20Reference) (OtherActor :type Actor%20Object%20Reference) (OtherComp :type Primitive%20Component%20Object%20Reference) (OtherBodyIndex :type Integer) (bFromSweep :type Boolean) (SweepResult :type Hit%20Result%20Structure%20%28by%20ref%29))
  ;[1 1 1] Get Buoyancy Actor List
)

(event OnComponentEndOverlap(BuoyancyVolume)
  (params (OverlappedComponent :type Primitive%20Component%20Object%20Reference) (OtherActor :type Actor%20Object%20Reference) (OtherComp :type Primitive%20Component%20Object%20Reference) (OtherBodyIndex :type Integer))
  ;[1 1 1] Get Buoyancy Actor List
)

(event EventBeginPlay)

(event EventTick
  (params (DeltaSeconds :type Float%20%28single-precision%29)))

(event EventParticleData
  (params (Data :type Array%20of%20Basic%20Particle%20Data%20Structures) (NiagaraSystem :type Niagara%20System%20Object%20Reference) (SimulationPositionOffset :type Vector%20%28by%20ref%29 :default "0, 0, 0")))

(fn ConstructionScript)