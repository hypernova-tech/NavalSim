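; Actor in the Waterline ocean content that tunes engine volumetric fog settings, named for underwater fog rendering.
; It runs a fixed set of r.VolumetricFog console commands covering grid resolution, depth distribution, temporal history, jitter and light function quality.
; The identical list runs in both the Construction Script and BeginPlay, so the global cvars apply in editor and at runtime, with nothing restoring previous values.
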(event EventBeginPlay
  (Development|ExecuteConsoleCommand (Utilities|String|Append "r.VolumetricFog.HistoryWeight " "0.2") 0)
  (Development|ExecuteConsoleCommand (Utilities|String|Append "r.VolumetricFog.ConservativeDepth " "1") 0)
  (Development|ExecuteConsoleCommand (Utilities|String|Append "r.VolumetricFog.DepthDistributionScale  " "80") 0)
  (Development|ExecuteConsoleCommand (Utilities|String|Append "r.VolumetricFog.GridPixelSize " "6") 0)
  (Development|ExecuteConsoleCommand (Utilities|String|Append "r.VolumetricFog.GridSizeZ " "160") 0)
  (Development|ExecuteConsoleCommand (Utilities|String|Append "r.VolumetricFog.HistoryMissSupersampleCount " "0") 0)
  (Development|ExecuteConsoleCommand (Utilities|String|Append "r.VolumetricFog.Jitter " "0") 0)
  (Development|ExecuteConsoleCommand (Utilities|String|Append "r.VolumetricFog.LightFunction.DirectionalLightSupersampleScale " "8") 0)
  (Development|ExecuteConsoleCommand (Utilities|String|Append "r.VolumetricFog.LightFunction.Resolution " "512") 0)
  (Development|ExecuteConsoleCommand (Utilities|String|Append "r.VolumetricFog.UpsampleJitterMultiplier " "1") 0))

(fn ConstructionScript
  (Development|ExecuteConsoleCommand (Utilities|String|Append "r.VolumetricFog.HistoryWeight " "0.2") 0)
  (Development|ExecuteConsoleCommand (Utilities|String|Append "r.VolumetricFog.ConservativeDepth " "1") 0)
  (Development|ExecuteConsoleCommand (Utilities|String|Append "r.VolumetricFog.DepthDistributionScale  " "80") 0)
  (Development|ExecuteConsoleCommand (Utilities|String|Append "r.VolumetricFog.GridPixelSize " "6") 0)
  (Development|ExecuteConsoleCommand (Utilities|String|Append "r.VolumetricFog.GridSizeZ " "160") 0)
  (Development|ExecuteConsoleCommand (Utilities|String|Append "r.VolumetricFog.HistoryMissSupersampleCount " "0") 0)
  (Development|ExecuteConsoleCommand (Utilities|String|Append "r.VolumetricFog.Jitter " "0") 0)
  (Development|ExecuteConsoleCommand (Utilities|String|Append "r.VolumetricFog.LightFunction.DirectionalLightSupersampleScale " "8") 0)
  (Development|ExecuteConsoleCommand (Utilities|String|Append "r.VolumetricFog.LightFunction.Resolution " "512") 0)
  (Development|ExecuteConsoleCommand (Utilities|String|Append "r.VolumetricFog.UpsampleJitterMultiplier " "1") 0))